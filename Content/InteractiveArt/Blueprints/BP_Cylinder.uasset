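; BP_Cylinder is an interactive art piece whose centre tube, line and decal react to how far and in which direction PCAnchor sits from BaseMesh.
; Each Tick, beyond a small distance threshold, it eases the tube's height from distance and its yaw from direction using FInterpTo.
; The same vector drives the RotDecal dynamic material's emission and stretches and yaws LineStart along the base-to-anchor axis.
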(event EventTick
  (params (DeltaSeconds :type Float%20%28single-precision%29))
  (if (> (.Distance (CallFunction|GetBaseandAnchor false 1.0)) 2.0)
    (Variables|Default|SetDeltaTime DeltaSeconds)
    (CallFunction|SetCenterTubeLocationZ (.Distance (CallFunction|GetBaseandAnchor false 1.0)))
    (CallFunction|SetCenterTubeRotationZ (.RawVector (CallFunction|GetBaseandAnchor true 1.0)))
    (CallFunction|SetTubeDecalEmissionbyDistance (.Distance (CallFunction|GetBaseandAnchor false 1.0)))
    (CallFunction|SetLineRelativeScale3d)
    (CallFunction|SetLineWorldRotation)))

(event EventBeginPlay
  (bind _returnvalue (Rendering|Material|CreateDynamicMaterialInstance (Variables|Default|GetRotDecal) :!class /Script/Engine.DecalComponent))
  (Variables|Default|SetTubeDecalMaterial _returnvalue))

(fn ConstructionScript)

(fn GetBaseandAnchor
  (params (IsNormalized :type Boolean) (Scalar :type Float%20%28double-precision%29))
  (bind _basemesh (Variables|Default|GetBaseMesh))
  (bind _pc_anchor (Variables|Default|GetPC_Anchor))
  (bind _returnvalue (Transformation|GetWorldLocation _pc_anchor))
  (bind _returnvalue_2 (Transformation|GetWorldLocation _basemesh))
  (bind _returnvalue_3 (- _returnvalue _returnvalue_2))
  (return (Math|Vector|VectorLength _returnvalue_3) (* (select IsNormalized (Math|Vector|Normalize _returnvalue_3) _returnvalue_3) Scalar)))

(fn SetCenterTubeLocationZ
  (params (Value :type Float%20%28double-precision%29))
  (bind _output_get (Variables|Default|SetCurrentPositionZ (Math|Interpolation|FInterpTo (Variables|Default|GetCurrentPositionZ) (Math|Float|MapRangeClamped Value 3.0 125.0 0.0 145.0) (Variables|Default|GetDeltaTime) (Variables|Default|GetTubeMovementSpeed))))
  (Transformation|SetRelativeLocation (Variables|Default|GetTubeMesh) (Math|Vector|MakeVector 0.0 0.0 _output_get) false false))

(fn SetCenterTubeRotationZ
  (params (RawVector :type Vector%20%28by%20ref%29))
  (bind _output_get (Variables|Default|SetCurrentTubeRotZ (Math|Interpolation|FInterpTo (Variables|Default|GetCurrentTubeRotZ) (.Yaw (Math|Rotator|BreakRotator (Math|Rotator|MakeRotfromX RawVector))) (Variables|Default|GetDeltaTime) (Variables|Default|GetTubeRotationSpeed))))
  (Transformation|SetWorldRotation (Variables|Default|GetTubeMesh) (Math|Rotator|MakeRotator 0.0 0.0 _output_get) false false))

(fn SetTubeDecalEmissionbyDistance
  (params (Distance :type Float%20%28double-precision%29))
  (Rendering|Material|SetScalarParameterValue (Variables|Default|GetTubeDecalMaterial) "EmissionAmount" (Math|Float|MapRangeClamped Distance 2.0 125.0 0.0 4.0) :!class /Script/Engine.MaterialInstanceDynamic))

(fn SetLineRelativeScale3d
  (Transformation|SetRelativeScale3D (Variables|Default|GetLineStart) (Math|Vector|MakeVector (/ (.Distance (CallFunction|GetBaseandAnchor false 1.0)) 1e+01) 1.0 1.0)))

(fn SetLineWorldRotation
  (Transformation|SetWorldRotation (Variables|Default|GetLineStart) (Math|Rotator|MakeRotator 0.0 0.0 (.Yaw (Math|Rotator|BreakRotator (Math|Rotator|MakeRotfromX (.RawVector (CallFunction|GetBaseandAnchor true -1.0)))))) false false))