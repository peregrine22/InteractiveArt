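; BP_OSC is an actor that receives touch input over OSC for the interactive art project.
; On BeginPlay it starts an OSC server on a hardcoded IP and port, binding its message event.
; Incoming messages are routed by last address segment: touch count triggers press or release on Player.
; First-touch coordinates become a negated, PucX-scaled vector stored in OscXYPosition and printed for debugging.
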(event Custom|OSC_In
  (params (Message :type OSC%20Message%20Structure%20%28by%20ref%29) (IPAddress :type String) (Port :type Integer))
  (bind _player (Variables|Default|GetPlayer))
  (bind _output_get (Variables|Default|SetOscMessage Message))
  (bind _returnvalue (Class|OSCManager|GetOSCMessageAddress _output_get))
  (bind _returnvalue_2 (Class|OSCManager|GetOSCAddressFullPath _returnvalue))
  (switch string (.RightS (Utilities|String|Split _returnvalue_2 "/" "IgnoreCase" "FromEnd"))
    (:touchcount
      (bind _value (Class|OSCManager|GetInt32 (Variables|Default|GetOscMessage)))
      (if (== _value 1)
        (Default|OSCTouchPressed _player)
        (else
          (Default|OSCTouchReleased _player))))
    (:touch0
      (bind _value_2 (Class|OSCManager|GetFloat (Variables|Default|GetOscMessage)))
      (bind _value_3 (Class|OSCManager|GetFloat (Variables|Default|GetOscMessage) 1))
      (bind _output_get_2 (Variables|Default|SetOscXYPosition (* (Math|Vector|MakeVector _value_2 _value_3 0.0) (Variables|Default|GetPucX) (Math|Float|MakeLiteralFloat -1.0))))
      (Development|PrintString (Utilities|String|ToString(Vector) _output_get_2)))))

(event EventBeginPlay
  (bind _returnvalue (Class|OSCManager|CreateOSCServer "192.168.137.1" 1234 false true "" 0))
  (bind _output_get (Variables|Default|SetOscServer _returnvalue))
  (EventDispatchers|BindEventtoOnOscMessageReceived _output_get (EventDispatchers|CreateEvent :!event Custom|OSC_In)))

(event Collision|EventActorBeginOverlap
  (params (OtherActor :type Actor%20Object%20Reference)))

(event EventTick
  (params (DeltaSeconds :type Float%20%28single-precision%29)))

(fn ConstructionScript)