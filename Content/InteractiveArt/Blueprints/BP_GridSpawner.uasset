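; BP_GridSpawner spawns a grid of BP_Cylinder actors when play begins.
; The construction script builds static mesh components as placeholders, using X and Y counts and a spacing value.
; Its centering offset swaps the X and Y counts, so only square grids center on the origin.
; BeginPlay spawns a cylinder at each placeholder's world transform, then destroys the placeholders.
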(event EventBeginPlay
  (for _array_element (Variables|Default|GetSpawnMeshArray)
    (Game|SpawnActorfromClass "/Game/InteractiveArt/Blueprints/BP_Cylinder.BP_Cylinder_C" (Transformation|GetWorldTransform _array_element) "AlwaysSpawn" "MultiplyWithRoot" 0 0))
  (for _array_element_2 (Variables|Default|GetSpawnMeshArray)
    (Components|DestroyComponent _array_element_2)))

(fn ConstructionScript
  (Utilities|Array|Clear (Variables|Default|GetSpawnMeshArray))
  (for _index (range 0 (- (Variables|Default|GetMaxXAmount) 1))
    (Variables|Default|SetIndexX _index)
    (for _index_2 (range 0 (- (Variables|Default|GetMaxYAmount) 1))
      (Variables|Default|SetIndexY _index_2)
      (bind _returnvalue (AddComponent|AddStaticMeshComponent false (Math|Transform|MakeTransform (- (Math|Vector|MakeVector (* (Variables|Default|GetIndexX) (Variables|Default|GetSpasingBetweenInstances)) (* (Variables|Default|GetIndexY) (Variables|Default|GetSpasingBetweenInstances)) 0.0) (Math|Vector|MakeVector (/ (* (- (Variables|Default|GetMaxYAmount) 1) (Variables|Default|GetSpasingBetweenInstances)) 2.0) (/ (* (- (Variables|Default|GetMaxXAmount) 1) (Variables|Default|GetSpasingBetweenInstances)) 2.0) 0.0)))))
      (Utilities|Array|Add (Variables|Default|GetSpawnMeshArray) _returnvalue))))