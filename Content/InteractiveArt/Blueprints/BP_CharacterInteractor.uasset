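; Player-controlled interactor for an interactive art piece that moves a Puc actor via OSC touch or mouse input.
; In OSC mode it spawns BP_OSC, whose touch events gate Tick updates toward its XY position; otherwise Enhanced Input triggers updates toward the cursor, deprojected using camera height and flattened to Z=0.
; Movement is smoothed with VInterpTo; mouse mode also sets fullscreen, a 60 FPS cap and mappings including pause and quit.
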(event Custom|OSCTouchReleased
  (bind _returnvalue (Game|GetPlayerController 0))
  (bind (_worldlocation _worlddirection) (Game|Player|ConvertMouseLocationToWorldSpace _returnvalue))
  (Utilities|FlowControl|Gate true) ; enters at Close
)

(event Custom|OSCTouchPressed
  (bind _returnvalue (Game|GetPlayerController 0))
  (bind (_worldlocation _worlddirection) (Game|Player|ConvertMouseLocationToWorldSpace _returnvalue))
  (Utilities|FlowControl|Gate true) ; enters at Open
)

(event Input|EnhancedActionEvents|EnhancedInputActionIA_Action
  (params (ActionValue :type Boolean) (ElapsedSeconds :type Float%20%28double-precision%29) (TriggeredSeconds :type Float%20%28double-precision%29) (InputAction :type Input%20Action%20Object%20Reference :default "/Game/InteractiveArt/Input/IA_Action.IA_Action"))
  (bind _returnvalue (Game|GetPlayerController 0))
  (bind (_worldlocation _worlddirection) (Game|Player|ConvertMouseLocationToWorldSpace _returnvalue))
  (:Triggered
    (bind _output_get (Variables|Default|SetCurrentPucPosition (Math|Interpolation|VInterpTo (Variables|Default|GetCurrentPucPosition) (select (Variables|Default|GetIsOSCMode) (Variables|/Game/InteractiveArt/Blueprints/BP_OSC.BP_OSC_C|GetOscXYPosition (Variables|Default|GetBP_OSC)) (* (+ _worldlocation (* _worlddirection (.Z (Math|Vector|BreakVector (Transformation|GetWorldLocation (Variables|Default|GetCineCamera)))))) "1.000000,1.000000,0.000000")) (Variables|Default|GetDeltaTime) (Variables|Default|GetPucLocationInterpolationSpeed))))
    (Transformation|SetActorLocation (Variables|Default|GetPuc) _output_get false false)))

(event Input|EnhancedActionEvents|EnhancedInputActionIA_Escape
  (params (ActionValue :type Boolean) (ElapsedSeconds :type Float%20%28double-precision%29) (TriggeredSeconds :type Float%20%28double-precision%29) (InputAction :type Input%20Action%20Object%20Reference :default "/Game/InteractiveArt/Input/IA_Escape.IA_Escape"))
  (:Triggered
    (Game|QuitGame 0 "Quit" false)))

(event Input|EnhancedActionEvents|EnhancedInputActionIA_Pause
  (params (ActionValue :type Boolean) (ElapsedSeconds :type Float%20%28double-precision%29) (TriggeredSeconds :type Float%20%28double-precision%29) (InputAction :type Input%20Action%20Object%20Reference :default "/Game/InteractiveArt/Input/IA_Pause.IA_Pause"))
  (:Triggered
    (Utilities|FlowControl|FlipFlop
      (:A
        (Game|SetGamePaused true))
      (:B
        (Game|SetGamePaused false)))))

(event EventBeginPlay
  (Variables|Default|SetCurrentPucPosition (Transformation|GetActorLocation (Variables|Default|GetPuc)))
  (bind _asplayer_controller (Utilities|Casting|CastToPlayerController (Pawn|GetController)))
  (if (Variables|Default|GetIsOSCMode)
    (Variables|/Script/Engine.PlayerController|SetbShowMouseCursor _asplayer_controller false)
    (bind _returnvalue (Game|SpawnActorfromClass "/Game/InteractiveArt/Blueprints/BP_OSC.BP_OSC_C" (Math|Transform|MakeTransform "0, 0, 0") "AlwaysSpawn" "MultiplyWithRoot" 0 self 0))
    (Variables|Default|SetBP_OSC _returnvalue)
    (else
      (Variables|/Script/Engine.PlayerController|SetbShowMouseCursor _asplayer_controller true)
      (Utilities|IsValid (PlayerController|LocalPlayerSubsystems|GetEnhancedInputLocalPlayerSubsystem _asplayer_controller)
        (:Is%20Valid
          (Input|AddMappingContext (PlayerController|LocalPlayerSubsystems|GetEnhancedInputLocalPlayerSubsystem _asplayer_controller) "/Game/InteractiveArt/Input/IC_InteractiveArt.IC_InteractiveArt" 0 "(bIgnoreAllPressedKeysUntilRelease=True,bForceImmediately=False)")
          (Development|ExecuteConsoleCommand "fullscreen" 0)
          (Development|ExecuteConsoleCommand "t.MaxFps 60" 0))
        (:Is%20Not%20Valid
          (Development|PrintString "EIC not valid"))))))

(event EventTick
  (params (DeltaSeconds :type Float%20%28single-precision%29))
  (bind _returnvalue (Game|GetPlayerController 0))
  (bind (_worldlocation _worlddirection) (Game|Player|ConvertMouseLocationToWorldSpace _returnvalue))
  (Variables|Default|SetDeltaTime DeltaSeconds)
  (Utilities|FlowControl|Gate true
    (:Exit
      (bind _output_get (Variables|Default|SetCurrentPucPosition (Math|Interpolation|VInterpTo (Variables|Default|GetCurrentPucPosition) (select (Variables|Default|GetIsOSCMode) (Variables|/Game/InteractiveArt/Blueprints/BP_OSC.BP_OSC_C|GetOscXYPosition (Variables|Default|GetBP_OSC)) (* (+ _worldlocation (* _worlddirection (.Z (Math|Vector|BreakVector (Transformation|GetWorldLocation (Variables|Default|GetCineCamera)))))) "1.000000,1.000000,0.000000")) (Variables|Default|GetDeltaTime) (Variables|Default|GetPucLocationInterpolationSpeed))))
      (Transformation|SetActorLocation (Variables|Default|GetPuc) _output_get false false))))

(fn ConstructionScript)